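; Camera component for the BP_P_Plankton pawn that detaches its camera and follows in the Y/Z plane at a fixed X distance.
; Tick eases toward the clamped target, varying interp speed with pawn velocity, ZipCam and distance.
; UpdateUniversalBound resolves each directional limit from CameraBoundaries, favouring higher layers, then the smaller absolute limit on ties.
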(event EventBeginPlay
  (bind _asbp_p_plankton (Utilities|Casting|CastToBP_P_Plankton (Components|GetOwner)))
  (Variables|Components|SetPlayer_Char _asbp_p_plankton)
  (bind _output_get (Variables|Default|SetCamera (Actor|GetComponentbyClass (Components|GetOwner) "/Script/Engine.CameraComponent")))
  (Transformation|DetachFromComponent _output_get "KeepWorld" "KeepWorld" "KeepRelative" true)
  (Utilities|FlowControl|Delay 0.0)
  (Transformation|SetWorldLocation _output_get (Math|Vector|MakeVector (+ (* (Variables|Components|GetDefault_dis) -1.0) (.x (Transformation|GetActorLocation (Variables|Components|GetPlayer_Char)))) (.y (Transformation|GetActorLocation (Variables|Components|GetPlayer_Char))) (.z (Transformation|GetActorLocation (Variables|Components|GetPlayer_Char)))) false false))

(event EventTick
  (params (DeltaSeconds :type Float%20%28single-precision%29))
  (bind _camera (Variables|Default|GetCamera))
  (bind _camera_2 (Variables|Default|GetCamera))
  (bind _returnvalue (Transformation|GetWorldLocation _camera))
  (Transformation|SetWorldLocation _camera_2 (Math|Vector|MakeVector (.x (Transformation|GetWorldLocation _camera_2)) (Math|Interpolation|FInterpTo (.y (Transformation|GetWorldLocation (Variables|Default|GetCamera))) (.y (Utilities|CameraClamped)) (Utilities|Time|GetWorldDeltaSeconds) (Math|Float|SelectFloat (Math|Float|SelectFloat (select (not (Math|Float|NearlyEqual(Float) (.y (Variables|/Game/BP/PC_Pawn/BP_P_Plankton.BP_P_Plankton_C|GetMaxVelocity (Variables|Components|GetPlayer_Char))) 0.0 0.5)) 4.0 1.5) 1.0 (Variables|/Game/BP/PC_Pawn/BP_P_Plankton.BP_P_Plankton_C|GetZipCam (Variables|Components|GetPlayer_Char))) (Math|Float|Absolute(Float) (/ (Variables|Components|GetDefault_dis) (.y (- (Transformation|GetWorldLocation (Variables|Default|GetCamera)) (Utilities|CameraClamped))))) (> (Math|Float|Absolute(Float) (- (.y (Transformation|GetWorldLocation (Variables|Default|GetCamera))) (.y (Utilities|CameraClamped)))) (/ (Variables|Components|GetDefault_dis) 3.0)))) (Math|Interpolation|FInterpTo (.z (Transformation|GetWorldLocation (Variables|Default|GetCamera))) (.z (Utilities|CameraClamped)) (Utilities|Time|GetWorldDeltaSeconds) (Math|Float|SelectFloat 3.5 5.0 (Math|Boolean|ANDBoolean (< (.z (Variables|/Game/BP/PC_Pawn/BP_P_Plankton.BP_P_Plankton_C|GetMaxVelocity (Variables|Components|GetPlayer_Char))) -1.0) (> (- (.z _returnvalue) (.z (Utilities|CameraClamped))) 0.0) (> (- (.z _returnvalue) (.ReturnZ (Utilities|CameraUnbounded))) 0.0))))) false false))

(fn UpdateUniversalBound
  (for _array_element (Variables|CameraBounds|GetCameraBoundaries)
    (LocalVariables|SetCurrendBound _array_element)
    (bind _enumvalue (|ForEachE_Direction)
      (:LoopBody
        (if (Utilities|Select :Index _enumvalue :NewEnumerator0 (Variables|/Game/BP/PC_Pawn/CameraComponents/BP_CameraBoundary.BP_CameraBoundary_C|GetboxUp (LocalVariables|GetCurrendBound)) :NewEnumerator1 (Variables|/Game/BP/PC_Pawn/CameraComponents/BP_CameraBoundary.BP_CameraBoundary_C|GetboxDown (LocalVariables|GetCurrendBound)) :NewEnumerator2 (Variables|/Game/BP/PC_Pawn/CameraComponents/BP_CameraBoundary.BP_CameraBoundary_C|GetboxLeft (LocalVariables|GetCurrendBound)) :NewEnumerator3 (Variables|/Game/BP/PC_Pawn/CameraComponents/BP_CameraBoundary.BP_CameraBoundary_C|GetboxRight (LocalVariables|GetCurrendBound)))
          (if (> (Variables|/Game/BP/PC_Pawn/CameraComponents/BP_CameraBoundary.BP_CameraBoundary_C|GetLayer (LocalVariables|GetCurrendBound)) (Utilities|Select :Index _enumvalue :NewEnumerator0 (LocalVariables|GetLocalLayerNorth) :NewEnumerator1 (LocalVariables|GetLocalLayerSouth) :NewEnumerator2 (LocalVariables|GetLocalLayerWest) :NewEnumerator3 (LocalVariables|GetLocalLayerEast)))
            (|SetBy-RefVar (Utilities|Select :Index _enumvalue :NewEnumerator0 (LocalVariables|GetNorthLocalLim) :NewEnumerator1 (LocalVariables|GetSouthLocalLim) :NewEnumerator2 (LocalVariables|GetWestLocalLim) :NewEnumerator3 (LocalVariables|GetEastLocalLim)) (Utilities|Select :Index _enumvalue :NewEnumerator0 (Variables|/Game/BP/PC_Pawn/CameraComponents/BP_CameraBoundary.BP_CameraBoundary_C|GetNorthLimit (LocalVariables|GetCurrendBound)) :NewEnumerator1 (Variables|/Game/BP/PC_Pawn/CameraComponents/BP_CameraBoundary.BP_CameraBoundary_C|GetSouthLimit (LocalVariables|GetCurrendBound)) :NewEnumerator2 (Variables|/Game/BP/PC_Pawn/CameraComponents/BP_CameraBoundary.BP_CameraBoundary_C|GetWestLimit (LocalVariables|GetCurrendBound)) :NewEnumerator3 (Variables|/Game/BP/PC_Pawn/CameraComponents/BP_CameraBoundary.BP_CameraBoundary_C|GetEastLimit (LocalVariables|GetCurrendBound))) :!label _label)
            (|SetBy-RefVar (Utilities|Select :Index _enumvalue :NewEnumerator0 (LocalVariables|GetLocalLayerNorth) :NewEnumerator1 (LocalVariables|GetLocalLayerSouth) :NewEnumerator2 (LocalVariables|GetLocalLayerWest) :NewEnumerator3 (LocalVariables|GetLocalLayerEast)) (Variables|/Game/BP/PC_Pawn/CameraComponents/BP_CameraBoundary.BP_CameraBoundary_C|GetLayer (LocalVariables|GetCurrendBound)))
            (elif (== (Variables|/Game/BP/PC_Pawn/CameraComponents/BP_CameraBoundary.BP_CameraBoundary_C|GetLayer (LocalVariables|GetCurrendBound)) (Utilities|Select :Index _enumvalue :NewEnumerator0 (LocalVariables|GetLocalLayerNorth) :NewEnumerator1 (LocalVariables|GetLocalLayerSouth) :NewEnumerator2 (LocalVariables|GetLocalLayerWest) :NewEnumerator3 (LocalVariables|GetLocalLayerEast)))
              (if (< (Math|Float|Absolute(Float) (Utilities|Select :Index _enumvalue :NewEnumerator0 (Variables|/Game/BP/PC_Pawn/CameraComponents/BP_CameraBoundary.BP_CameraBoundary_C|GetNorthLimit (LocalVariables|GetCurrendBound)) :NewEnumerator1 (Variables|/Game/BP/PC_Pawn/CameraComponents/BP_CameraBoundary.BP_CameraBoundary_C|GetSouthLimit (LocalVariables|GetCurrendBound)) :NewEnumerator2 (Variables|/Game/BP/PC_Pawn/CameraComponents/BP_CameraBoundary.BP_CameraBoundary_C|GetWestLimit (LocalVariables|GetCurrendBound)) :NewEnumerator3 (Variables|/Game/BP/PC_Pawn/CameraComponents/BP_CameraBoundary.BP_CameraBoundary_C|GetEastLimit (LocalVariables|GetCurrendBound)))) (Math|Float|Absolute(Float) (Utilities|Select :Index _enumvalue :NewEnumerator0 (LocalVariables|GetNorthLocalLim) :NewEnumerator1 (LocalVariables|GetSouthLocalLim) :NewEnumerator2 (LocalVariables|GetWestLocalLim) :NewEnumerator3 (LocalVariables|GetEastLocalLim))))
                (goto _label))))))))
  (bind _enumvalue_2 (|ForEachE_Direction)
    (:LoopBody
      (|SetBy-RefVar (Utilities|Select :Index _enumvalue_2 :NewEnumerator0 (Variables|CameraBounds|GetNorthlim) :NewEnumerator1 (Variables|CameraBounds|GetSouthlim) :NewEnumerator2 (Variables|CameraBounds|GetWestlim) :NewEnumerator3 (Variables|CameraBounds|GetEastlim)) (Utilities|Select :Index _enumvalue_2 :NewEnumerator0 (LocalVariables|GetNorthLocalLim) :NewEnumerator1 (LocalVariables|GetSouthLocalLim) :NewEnumerator2 (LocalVariables|GetWestLocalLim) :NewEnumerator3 (LocalVariables|GetEastLocalLim))))))