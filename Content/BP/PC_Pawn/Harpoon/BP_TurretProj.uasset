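; BP_TurretProj is a turret projectile that damages and knocks back the Plankton pawn.
; BeginPlay applies its Velocity to ProjectileMovement and caches its owner as the Plankton target.
; A Despawn overlap destroys it, starts knockback and damages every Char_Health_Component actor, but compares its own overlapped component to the pawn's Painbox.
; Tick's intended five-second despawn tests per-frame DeltaSeconds, not accumulated lifetime.
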(event OnComponentBeginOverlap(Despawn)
  (params (OverlappedComponent :type Primitive%20Component%20Object%20Reference) (OtherActor :type Actor%20Object%20Reference) (OtherComp :type Primitive%20Component%20Object%20Reference) (OtherBodyIndex :type Integer) (bFromSweep :type Boolean) (SweepResult :type Hit%20Result%20Structure%20%28by%20ref%29))
  (bind _pc (Variables|Default|GetPC))
  (if (== OtherActor _pc)
    (if (== OverlappedComponent (Variables|/Game/BP/PC_Pawn/BP_P_Plankton.BP_P_Plankton_C|GetPainbox _pc))
      (Actor|DestroyActor)
      (Default|StartKnockBack (Variables|Default|GetPC))
      (bind _outactors (Actor|GetAllActorsOfClass "/Game/BP/Health_UI/Health_Ui/Health_System/Char_Health_Component.Char_Health_Component_C"))
      (for _array_element _outactors
        (Default|Damage _array_element)))))

(event Collision|EventActorBeginOverlap
  (params (OtherActor :type Actor%20Object%20Reference)))

(event EventTick
  (params (DeltaSeconds :type Float%20%28single-precision%29))
  (if (>= DeltaSeconds 5.0)
    (Actor|DestroyActor)))

(event EventBeginPlay
  (Variables|/Script/Engine.MovementComponent|SetVelocity (Variables|Default|GetProjectileMovement) (Variables|Default|GetVelocity))
  (bind _asbp_p_plankton (Utilities|Casting|CastToBP_P_Plankton (Components|GetOwner)))
  (Variables|Default|SetPC _asbp_p_plankton))

(fn ConstructionScript)