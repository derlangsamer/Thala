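; Box volume that defines camera limits on the Y/Z plane for the BP_P_Plankton pawn.
; The construction script derives North, South, East and West limits from the box extents, pushing any side flagged as a bridge out to a huge distance.
; Plankton overlaps add or remove it from the camera component's boundary list and update the universal bound.
; BeginPlay sweeps it away and back, apparently to refresh initial overlaps.
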(event OnComponentBeginOverlap(Box)
  (params (OverlappedComponent :type Primitive%20Component%20Object%20Reference) (OtherActor :type Actor%20Object%20Reference) (OtherComp :type Primitive%20Component%20Object%20Reference) (OtherBodyIndex :type Integer) (bFromSweep :type Boolean) (SweepResult :type Hit%20Result%20Structure%20%28by%20ref%29))
  (bind _asbp_p_plankton (Utilities|Casting|CastToBP_P_Plankton OtherActor))
  (Utilities|Array|AddUnique (Variables|/Game/BP/PC_Pawn/BP_CameraComponent.BP_CameraComponent_C|GetCameraBoundaries (Variables|/Game/BP/PC_Pawn/BP_P_Plankton.BP_P_Plankton_C|GetBP_CameraComponent _asbp_p_plankton)) self)
  (Default|UpdateUniversalBound (Variables|/Game/BP/PC_Pawn/BP_P_Plankton.BP_P_Plankton_C|GetBP_CameraComponent _asbp_p_plankton)))

(event OnComponentEndOverlap(Box)
  (params (OverlappedComponent :type Primitive%20Component%20Object%20Reference) (OtherActor :type Actor%20Object%20Reference) (OtherComp :type Primitive%20Component%20Object%20Reference) (OtherBodyIndex :type Integer))
  (bind _asbp_p_plankton (Utilities|Casting|CastToBP_P_Plankton OtherActor))
  (Utilities|Array|RemoveItem (Variables|/Game/BP/PC_Pawn/BP_CameraComponent.BP_CameraComponent_C|GetCameraBoundaries (Variables|/Game/BP/PC_Pawn/BP_P_Plankton.BP_P_Plankton_C|GetBP_CameraComponent _asbp_p_plankton)) self)
  (Default|UpdateUniversalBound (Variables|/Game/BP/PC_Pawn/BP_P_Plankton.BP_P_Plankton_C|GetBP_CameraComponent _asbp_p_plankton)))

(event EventBeginPlay
  (Transformation|AddActorLocalOffset "10000.000000, 0, 0" true false)
  (Utilities|FlowControl|Delay 0.0)
  (Transformation|AddActorLocalOffset "-10000.000000, 0, 0" true false))

(fn ConstructionScript
  (bind _returnvalue (Transformation|GetActorLocation))
  (bind _box (Variables|Default|GetBox))
  (bind _returnvalue_2 (Components|Box|GetScaledBoxExtent _box))
  (bind _enumvalue (|ForEachE_Direction)
    (:LoopBody
      (|SetBy-RefVar (Utilities|Select :Index _enumvalue :NewEnumerator0 (Variables|Default|GetNorthLimit) :NewEnumerator1 (Variables|Default|GetSouthLimit) :NewEnumerator2 (Variables|Default|GetWestLimit) :NewEnumerator3 (Variables|Default|GetEastLimit)) (+ (Utilities|Select :Index _enumvalue :NewEnumerator0 (.z _returnvalue) :NewEnumerator1 (.z _returnvalue) :NewEnumerator2 (.y _returnvalue) :NewEnumerator3 (.y _returnvalue)) (* (select (Utilities|Select :Index _enumvalue :NewEnumerator0 (Variables|Default|GetboxUpbridge) :NewEnumerator1 (Variables|Default|GetboxDownbridge) :NewEnumerator2 (Variables|Default|Getboxleftbridge) :NewEnumerator3 (Variables|Default|GetboxRightbridge)) 5e+07 (Utilities|Select :Index _enumvalue :NewEnumerator0 (.z _returnvalue_2) :NewEnumerator1 (.z _returnvalue_2) :NewEnumerator2 (.y _returnvalue_2) :NewEnumerator3 (.y _returnvalue_2))) (Utilities|Select :Index _enumvalue :NewEnumerator0 1.0 :NewEnumerator1 -1.0 :NewEnumerator2 -1.0 :NewEnumerator3 1.0)))))))