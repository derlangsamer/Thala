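; Harpoon component that fires a hook and cable from its owner toward a target, as a grapple for the player pawn.
; A Ready/Fire/Zip state blocks refiring; a hit starts Zip, where Tick applies force from ToHitLocation, whose direction math is unwired.
; The hook is destroyed near the player or on AniCancel.
; Its destruction removes the cable, resets to Ready and sets the BP_P_Plankton movement mode.
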(event EventTick
  (params (DeltaSeconds :type Float%20%28single-precision%29))
  ;[1 1 1] Player Zip
  (switch Utilities|FlowControl|Switch|SwitchonE_HarpoonStates (Variables|Default|GetHarpoonState)
    (:NewEnumerator2
      (bind _ascharacter (Utilities|Casting|CastToCharacter (Game|Player|GetPlayerPawn 0)))
      (Physics|AddForce (Variables|/Script/Engine.Character|GetCharacterMovement _ascharacter) (* (Utilities|ToHitLocation) 1e+04))
      ;[1 1 1] Depawner
      (if (< (Math|Vector|Distance(Vector) (Transformation|GetActorLocation (Variables|Default|GetHarpoonHook)) (Transformation|GetActorLocation (Game|Player|GetPlayerPawn 0))) 2.5e+02)
        (Actor|DestroyActor (Variables|Default|GetHarpoonHook))
        (Development|PrintString (Utilities|GetDisplayName (Variables|Default|GetHarpoonHook)))))))

(fn HarpoonCurrentState
  ;[1 1 1] State Checker
  (return (Utilities|Select :Index (Variables|Default|GetHarpoonState) :NewEnumerator0 false :NewEnumerator1 true :NewEnumerator2 true)))

(fn Fire
  (params (TarLoc :type Vector) (PC_Offset :type Vector))
  (bind _returnvalue (Components|GetOwner))
  (bind _returnvalue_2 (Transformation|GetActorTransform _returnvalue))
  (bind _returnvalue_3 (Transformation|GetActorLocation _returnvalue))
  (bind _returnvalue_4 (Math|Transform|TransformDirection _returnvalue_2 PC_Offset))
  (bind _returnvalue_5 (+ _returnvalue_4 _returnvalue_3))
  ;[1 1 1] State Check
  (if (not (CallFunction|HarpoonCurrentState))
    (Variables|Default|SetHarpoonState "NewEnumerator1")
    (LocalVariables|SetShotVector (Math|Vector|Normalize (- TarLoc _returnvalue_5)))
    (bind _returnvalue_6 (Game|SpawnActorfromClass "/Game/BP/PC_Pawn/Harpoon/BP_Harpoon.BP_Harpoon_C" (Math|Transform|MakeTransform _returnvalue_5 "0, 0, 0" "1,1,1") "Undefined" 0 (* (LocalVariables|GetShotVector) (LocalVariables|GetSpeed)) 0))
    ;[1 1 1] Custom On Hit
    (bind _output_get (Variables|Default|SetHarpoonHook _returnvalue_6))
    (Collision|BindEventtoOnActorHit _output_get (EventDispatchers|CreateEvent :!event OnHarpoonHit))
    ;[1 1 1] Despawn/Cleanup
    (Game|BindEventtoOnDestroyed (Variables|Default|GetHarpoonHook) (EventDispatchers|CreateEvent :!event HarpoonDespawn))
    ;[1 1 1] Harpoon Cable Spawner and Attach logic
    (bind _returnvalue_7 (Game|SpawnActorfromClass "/Game/BP/PC_Pawn/Harpoon/BP_Cable.BP_Cable_C" (Math|Transform|MakeTransform _returnvalue_5 (Math|Rotator|MakeRotfromX (LocalVariables|GetShotVector)) "1,1,1") "Undefined" 0 0))
    (bind _output_get_2 (Variables|Default|SetCableManagement _returnvalue_7))
    (Transformation|AttachActorToActor _output_get_2 (Game|Player|GetPlayerPawn 0) "None" "KeepWorld" "KeepWorld" "KeepWorld" true)
    (Class|CableComponent|SetAttachEndto (Variables|/Script/CableComponent.CableActor|GetCableComponent (Variables|Default|GetCableManagement)) (Variables|Default|GetHarpoonHook) "None" "None")
    (Variables|/Script/CableComponent.CableComponent|SetEndLocation (Variables|/Script/CableComponent.CableActor|GetCableComponent (Variables|Default|GetCableManagement)) "0, 0, 0")))

(fn OnHarpoonHit
  (params (SelfActor :type Actor%20Object%20Reference) (OtherActor :type Actor%20Object%20Reference) (NormalImpulse :type Vector) (Hit :type Hit%20Result%20Structure%20%28by%20ref%29))
  ;[1 1 1] Removing Physics on Player to have a clean zip
  (Variables|Default|SetHarpoonState "NewEnumerator2")
  (Development|PrintString "Hello"))

(fn HarpoonDespawn
  (params (DestroyedActor :type Actor%20Object%20Reference))
  ;[1 1 1] Harpoon Cleanup
  (Variables|Default|SetHarpoonHook 0)
  (Variables|Default|SetHarpoonState "NewEnumerator0")
  (Utilities|FlowControl|Sequence
    (:then_0
      (bind _cablemanagement (Variables|Default|GetCableManagement)
        (:then
          (Actor|DestroyActor _cablemanagement)
          (Variables|Default|SetCableManagement 0))
        (:else)))
    (:then_1
      ;[1 1 1] Reset Character Control resetting Velocity
      (bind _asbp_p_plankton (Utilities|Casting|CastToBP_P_Plankton (Game|Player|GetPlayerPawn 0)))
      (Variables|/Game/BP/PC_Pawn/BP_P_Plankton.BP_P_Plankton_C|SetMovementMode _asbp_p_plankton "NewEnumerator3"))))

(fn AniCancel
  (bind _harpoonhook (Variables|Default|GetHarpoonHook)
    (:then
      (Actor|DestroyActor _harpoonhook))
    (:else)))