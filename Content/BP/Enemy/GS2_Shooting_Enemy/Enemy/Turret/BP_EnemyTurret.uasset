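; BP_EnemyTurret is an enemy turret that turns its Cone component to track the first player's pawn.
; Every Tick calls UpdateRotation, which interpolates the cone's world rotation toward the look-at angle at RotationSpeed, with zero roll and unrestricted yaw.
; Pitch is capped by BarrelLength through a Min, then clamped to a fixed range.
; FireWeapons is a stub that only waits FireInterval, with nothing calling it here.
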(event Custom|UpdateRotation
  (bind _returnvalue (Game|Player|GetPlayerPawn 0))
  (bind _cone (Variables|Default|GetCone))
  (bind _returnvalue_2 (Transformation|GetWorldLocation _cone))
  (bind _returnvalue_3 (Transformation|GetActorLocation _returnvalue))
  (bind _returnvalue_4 (Math|Rotator|FindLookatRotation _returnvalue_2 _returnvalue_3))
  (bind (_roll _pitch _yaw) (Math|Rotator|BreakRotator _returnvalue_4))
  (Transformation|SetWorldRotation (Variables|Default|GetCone) (Math|Interpolation|RInterpTo (Transformation|GetWorldRotation (Variables|Default|GetCone)) (Math|Rotator|MakeRotator 0.0 (Math|Float|ClampAngle (Math|Float|Min(Float) _pitch (Variables|TurretSettings|GetBarrelLength)) -1e+01 35.0) _yaw) (Variables|Components|GetDeltaTime) (Variables|TurretSettings|GetRotationSpeed)) false false))

(event Custom|FireWeapons
  (Utilities|FlowControl|Delay (Variables|TurretSettings|GetFireInterval)))

(event EventTick
  (params (DeltaSeconds :type Float%20%28single-precision%29))
  (Variables|Components|SetDeltaTime DeltaSeconds)
  (CallFunction|UpdateRotation))

(fn ConstructionScript)