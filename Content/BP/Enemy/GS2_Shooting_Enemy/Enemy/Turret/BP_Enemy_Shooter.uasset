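; BP_Enemy_Shooter is a turret enemy that shoots projectiles at the Plankton player pawn when it sees it.
; PawnSensing sightings rotate the whole actor to face the target, then spawn a BP_TurretProj at the ProjectileSpawnLocation transform.
; The projectile's mesh is launched by a physics impulse along the Cube's forward vector, scaled by ShootAmount.
; A SpawnProjectile flag with a short delay throttles the fire rate.
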(event OnSeePawn(PawnSensing)
  (params (Pawn :type Pawn%20Object%20Reference))
  (bind _asbp_p_plankton (Utilities|Casting|CastToBP_P_Plankton Pawn))
  (Utilities|FlowControl|Sequence
    (:then_0
      (Transformation|SetActorRotation (Math|Rotator|FindLookatRotation (Transformation|GetActorLocation) (Transformation|GetActorLocation _asbp_p_plankton))))
    (:then_1
      (if (Variables|Default|GetSpawnProjectile)
        (bind _returnvalue (Game|SpawnActorfromClass "/Game/BP/PC_Pawn/Harpoon/BP_TurretProj.BP_TurretProj_C" (Transformation|GetWorldTransform (Variables|Default|GetProjectileSpawnLocation)) "Undefined" 0 "0.000000,0.000000,0.000000" 0))
        (Physics|AddImpulse (Variables|/Game/BP/PC_Pawn/Harpoon/BP_TurretProj.BP_TurretProj_C|GetStaticMesh _returnvalue) (* (Math|Vector|GetForwardVector (Variables|Default|GetCube)) (Variables|Default|GetShootAmount)) "None" false)
        (Variables|Default|SetSpawnProjectile false)
        (Utilities|FlowControl|Delay 1.0)
        (Variables|Default|SetSpawnProjectile true)))))

(fn ConstructionScript)