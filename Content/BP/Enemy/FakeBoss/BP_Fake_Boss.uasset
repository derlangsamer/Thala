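; BP_Fake_Boss is an enemy that travels along a spline while facing the player's plankton pawn.
; A timeline started on BeginPlay drives the capsule along the spline, and Tick overrides rotation to look at the player.
; The player's first overlap with the TooClose trigger plays a floating montage and sets the "Advance Points" blackboard flag on its AI controller.
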(event OnComponentBeginOverlap(TooClose)
  (params (OverlappedComponent :type Primitive%20Component%20Object%20Reference) (OtherActor :type Actor%20Object%20Reference) (OtherComp :type Primitive%20Component%20Object%20Reference) (OtherBodyIndex :type Integer) (bFromSweep :type Boolean) (SweepResult :type Hit%20Result%20Structure%20%28by%20ref%29))
  (if (== OtherActor (Variables|Default|GetPC))
    (Utilities|FlowControl|DoOnce false
      (:Completed
        (Animation|PlayAnimMontage "/Game/Animations/FishBoss/BossAnimations/Floating_Montage.Floating_Montage" 1.0 "None")
        (Development|PrintString "Too Close")
        (AI|Components|Blackboard|SetValueasBool (AI|GetBlackboard (AI|GetAIController self)) (Utilities|Name|MakeLiteralName "Advance Points") true)))))

(event EventBeginPlay
  (bind _spline (Variables|Default|GetSpline))
  (bind _asbp_p_plankton (Utilities|Casting|CastToBP_P_Plankton (Game|Player|GetPlayerPawn 0)))
  (Variables|Default|SetPC _asbp_p_plankton)
  (bind _newtrack_0 (Timeline|Timeline_0 PlayFromStart)
    (:Update
      (Transformation|SetWorldTransform (Variables|Collision|GetCapsuleComponent) (Math|Transform|MakeTransform (Spline|GetLocationatDistanceAlongSpline _spline (* (Spline|GetSplineLength _spline) _newtrack_0) "World") (Spline|GetRotationatDistanceAlongSpline (Variables|Default|GetSpline) (* (Spline|GetSplineLength _spline) _newtrack_0) "Local")) false false))))

(event EventTick
  (params (DeltaSeconds :type Float%20%28single-precision%29))
  (Transformation|SetActorRotation (Math|Rotator|FindLookatRotation (Transformation|GetActorLocation self) (Transformation|GetActorLocation (Variables|Default|GetPC)))))

(fn ConstructionScript)