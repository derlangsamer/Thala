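; BP_FakeBossSpline is a spline path actor that guides the fake boss along a curve.
; BeginPlay positions and rotates the SplineEnd component from spline data, then caches its owner as BP_Fake_Boss.
; BeginSpline snaps the boss onto the nearest spline point and registers itself on the boss, while EndSpline clears that state.
; While StartTick is set, Tick locks the boss's horizontal position to the spline, preserving height.
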(event Custom|BeginSpline
  (bind _pc (Variables|Default|GetPC))
  (Variables|/Game/BP/Enemy/FakeBoss/BP_Fake_Boss.BP_Fake_Boss_C|SetInSpline _pc true)
  (Variables|/Game/BP/Enemy/FakeBoss/BP_Fake_Boss.BP_Fake_Boss_C|SetCurveSplineRef _pc self)
  (Transformation|SetWorldLocation (Variables|/Script/Engine.Character|GetCapsuleComponent (Variables|Default|GetPC)) (Spline|FindLocationClosesttoWorldLocation (Variables|Default|GetSpline) (Transformation|GetWorldLocation (Variables|/Script/Engine.Character|GetCapsuleComponent (Variables|Default|GetPC))) "World") false false))

(event Custom|EndSpline
  (bind _pc (Variables|Default|GetPC))
  (Variables|/Game/BP/Enemy/FakeBoss/BP_Fake_Boss.BP_Fake_Boss_C|SetInSpline _pc false)
  (Variables|/Game/BP/Enemy/FakeBoss/BP_Fake_Boss.BP_Fake_Boss_C|SetCurveSplineRef _pc 0))

(event EventBeginPlay
  (bind _splineend (Variables|Default|GetSplineEnd))
  (bind _splineend_2 (Variables|Default|GetSplineEnd))
  (bind _spline (Variables|Default|GetSpline))
  (bind _spline_2 (Variables|Default|GetSpline))
  (bind _returnvalue (Transformation|GetWorldLocation _splineend_2))
  (bind _returnvalue_2 (Spline|FindLocationClosesttoWorldLocation _spline _returnvalue "Local"))
  (bind (_x _y _z) (Class|KismetMathLibrary|BreakVector3f _returnvalue_2))
  (Transformation|SetWorldLocation _splineend (Math|Vector|MakeVector _x (+ _y 5e+01) _z) false false)
  (Transformation|SetWorldRotation _splineend (Spline|GetRotationatSplinePoint _spline_2 (Spline|GetNumberOfSplinePoints _spline_2) "Local") false false)
  (bind _asbp_fake_boss (Utilities|Casting|CastToBP_Fake_Boss (Components|GetOwner)))
  (Variables|Default|SetPC _asbp_fake_boss))

(event EventTick
  (params (DeltaSeconds :type Float%20%28single-precision%29))
  (bind _spline (Variables|Default|GetSpline))
  (bind _pc (Variables|Default|GetPC))
  (bind _capsulecomponent (Variables|/Script/Engine.Character|GetCapsuleComponent _pc))
  (bind _returnvalue (Transformation|GetWorldLocation _capsulecomponent))
  (bind _returnvalue_2 (Spline|FindLocationClosesttoWorldLocation _spline _returnvalue "World"))
  (if (Variables|Default|GetStartTick)
    (Transformation|SetWorldLocation (Variables|/Script/Engine.Character|GetCapsuleComponent (Variables|Default|GetPC)) (Math|Vector|MakeVector (.x _returnvalue_2) (.y _returnvalue_2) (.Z (Class|KismetMathLibrary|BreakVector3f _returnvalue))) false false)))

(fn ConstructionScript)