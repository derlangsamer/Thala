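; BP_SnailProj is an enemy projectile that launches along its local velocity at spawn and hurts the Plankton player.
; Overlapping the player's Painbox sets the knockback origin, starts knockback, destroys the projectile and calls Damage on every Char_Health_Component actor.
; Other overlaps destroy it, except itself and several Goomba, turret and Crunchy enemy types.
; Tick repeatedly makes its sphere ignore the AI_Crunchy actors cached at BeginPlay while moving.
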(event OnComponentBeginOverlap(Sphere)
  (params (OverlappedComponent :type Primitive%20Component%20Object%20Reference) (OtherActor :type Actor%20Object%20Reference) (OtherComp :type Primitive%20Component%20Object%20Reference) (OtherBodyIndex :type Integer) (bFromSweep :type Boolean) (SweepResult :type Hit%20Result%20Structure%20%28by%20ref%29))
  (bind _pc (Variables|Default|GetPC))
  (if (== OtherActor _pc)
    (if (== OtherComp (Variables|/Game/BP/PC_Pawn/BP_P_Plankton.BP_P_Plankton_C|GetPainbox _pc))
      (Variables|/Game/BP/PC_Pawn/BP_P_Plankton.BP_P_Plankton_C|SetKnockbackOrigin (Variables|Default|GetPC) (Transformation|GetActorLocation))
      (Actor|DestroyActor)
      (Default|StartKnockBack (Variables|Default|GetPC))
      (bind _outactors (Actor|GetAllActorsOfClass "/Game/BP/Health_UI/Health_Ui/Health_System/Char_Health_Component.Char_Health_Component_C"))
      (for _array_element _outactors
        (Default|Damage _array_element)))
    (elif (Math|Boolean|ANDBoolean (!= self OtherActor) (!= OtherActor "/Game/BP/Enemy/AI_GoombaV2.AI_GoombaV2") (!= OtherActor "/Game/BP/Enemy/AI_TurretTripleShot.AI_TurretTripleShot") (!= OtherActor "/Game/BP/Enemy/AI_GoombaV_3xs.AI_GoombaV_3xs") (!= OtherActor "/Game/BP/Enemy/AI_Crunchy.AI_Crunchy"))
      (Actor|DestroyActor))))

(event EventTick
  (params (DeltaSeconds :type Float%20%28single-precision%29))
  (for _array_element (Variables|Default|GetAs%20AI%20Crunchy)
    (Collision|IgnoreActorwhenMoving (Variables|Default|GetSphere) _array_element true)))

(event EventBeginPlay
  (Game|Components|ProjectileMovement|SetVelocityinLocalSpace (Variables|Default|GetProjectileMovement) (Variables|Default|GetProjectile%20Speed))
  (bind _asbp_p_plankton (Utilities|Casting|CastToBP_P_Plankton (Game|Player|GetPlayerPawn 0)))
  (Variables|Default|SetPC _asbp_p_plankton)
  (bind _outactors (Actor|GetAllActorsOfClass "/Game/BP/Enemy/AI_Crunchy.AI_Crunchy_C"))
  (Variables|Default|SetAs%20AI%20Crunchy _outactors))

(fn ConstructionScript)