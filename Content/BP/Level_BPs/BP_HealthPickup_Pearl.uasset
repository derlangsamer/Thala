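; BP_HealthPickup_Pearl is a pearl health pickup for the plankton player pawn.
; On BeginPlay it caches the pawn and starts a timeline that animates the sphere's height from its starting position.
; The first overlap by that pawn calls Heal repeatedly on Char_Health_Component actors found through GetAllActorsOfClass, rather than through the pawn.
; The pickup plays a sound and destroys itself inside that same loop.
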(event OnComponentBeginOverlap(Sphere1)
  (params (OverlappedComponent :type Primitive%20Component%20Object%20Reference) (OtherActor :type Actor%20Object%20Reference) (OtherComp :type Primitive%20Component%20Object%20Reference) (OtherBodyIndex :type Integer) (bFromSweep :type Boolean) (SweepResult :type Hit%20Result%20Structure%20%28by%20ref%29))
  (if (== OtherActor (Variables|Default|GetPC))
    (Utilities|FlowControl|DoOnce false
      (:Completed
        (bind _outactors (Actor|GetAllActorsOfClass "/Game/BP/Health_UI/Health_Ui/Health_System/Char_Health_Component.Char_Health_Component_C"))
        (for _array_element _outactors
          (Default|Heal _array_element)
          (Default|Heal _array_element)
          (Default|Heal _array_element)
          (Default|Heal _array_element)
          (Default|Heal _array_element)
          (Default|Heal _array_element)
          (Default|Heal _array_element)
          (Default|Heal _array_element)
          (Default|Heal _array_element)
          (Audio|PlaySoundatLocation 0 (Transformation|GetActorLocation) "0, 0, 0" 1.0 1.0 0.0 0 0 0 0)
          (Actor|DestroyActor))))))

(event EventBeginPlay
  (bind _sphere (Variables|Default|GetSphere))
  (bind _returnvalue (Transformation|GetWorldLocation _sphere))
  (bind _asbp_p_plankton (Utilities|Casting|CastToBP_P_Plankton (Game|Player|GetPlayerPawn 0)))
  (Variables|Default|SetPC _asbp_p_plankton)
  (Variables|Default|SetStarting%20Position (Transformation|GetWorldLocation (Variables|Default|GetSphere)))
  (bind _newtrack_0 (Timeline|Timeline_0 Play)
    (:Update
      (Transformation|SetWorldLocation _sphere (Math|Vector|MakeVector (.x _returnvalue) (.y _returnvalue) (Math|Float|Lerp (.z (Variables|Default|GetStarting%20Position)) (+ (.z (Transformation|GetWorldLocation (Variables|Default|GetSphere))) 2.0) _newtrack_0)) false false))))

(event Collision|EventActorBeginOverlap
  (params (OtherActor :type Actor%20Object%20Reference)))

(event EventTick
  (params (DeltaSeconds :type Float%20%28single-precision%29)))

(fn ConstructionScript)