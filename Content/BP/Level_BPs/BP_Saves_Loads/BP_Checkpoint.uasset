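; BP_Checkpoint is a checkpoint actor that saves a respawn transform when the BP_P_Plankton player overlaps it.
; On overlap, it loads the existing BP_SaveGame slot or creates a new save object.
; It stores its own location, raised slightly with zeroed rotation, as the Checkpoint and writes the slot on every overlap.
; A DoOnce limits the checkpoint sound, played at world origin, to the first save.
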(event OnComponentBeginOverlap(CheckpointOverlap)
  (params (OverlappedComponent :type Primitive%20Component%20Object%20Reference) (OtherActor :type Actor%20Object%20Reference) (OtherComp :type Primitive%20Component%20Object%20Reference) (OtherBodyIndex :type Integer) (bFromSweep :type Boolean) (SweepResult :type Hit%20Result%20Structure%20%28by%20ref%29))
  (bind _save_name (Variables|Default|GetSave%20Name))
  (Utilities|Casting|CastToBP_P_Plankton OtherActor)
  (bind _returnvalue (SaveGame|DoesSaveGameExist _save_name))
  (if _returnvalue
    (bind _returnvalue_2 (SaveGame|LoadGamefromSlot _save_name))
    (bind _asbp_save_game (Utilities|Casting|CastToBP_SaveGame _returnvalue_2))
    (Variables|Default|SetSavegameRef _asbp_save_game)
    (else
      (bind _returnvalue_3 (SaveGame|CreateSaveGameObject "/Game/BP/Level_BPs/BP_Saves_Loads/BP_SaveGame.BP_SaveGame_C"))
      (Variables|Default|SetSavegameRef _returnvalue_3)))
  (Variables|/Game/BP/Level_BPs/BP_Saves_Loads/BP_SaveGame.BP_SaveGame_C|SetCheckpoint (Variables|Default|GetSavegameRef) (Math|Transform|MakeTransform (+ (.location (Transformation|GetActorTransform)) "0, 0,10.000000")))
  (SaveGame|SaveGametoSlot (Variables|Default|GetSavegameRef) (Variables|Default|GetSave%20Name))
  (Utilities|FlowControl|DoOnce false
    (:Completed
      (Audio|PlaySoundatLocation "/Game/AudioAssets/Checkpoint.Checkpoint" "0, 0, 0" "0, 0, 0" 1.0 1.0 0.0 0 0 0))))

(fn ConstructionScript)