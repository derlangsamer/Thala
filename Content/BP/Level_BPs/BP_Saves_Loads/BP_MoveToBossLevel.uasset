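; BP_MoveToBossLevel is a trigger that sends the player's plankton pawn to Berni_BossLevel.
; When the cached BP_P_Plankton overlaps component R, a flag makes Tick zero the pawn's MaxVelocity and AddVelocity every frame, freezing it.
; The overlap also sets EventEnd on the owning actor if it is a Boss_Chase, prints a message, and opens the boss level after a short delay.
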(event OnComponentBeginOverlap(r)
  (params (OverlappedComponent :type Primitive%20Component%20Object%20Reference) (OtherActor :type Actor%20Object%20Reference) (OtherComp :type Primitive%20Component%20Object%20Reference) (OtherBodyIndex :type Integer) (bFromSweep :type Boolean) (SweepResult :type Hit%20Result%20Structure%20%28by%20ref%29))
  (bind _as_bp_p_plankton (Variables|Default|GetAs%20BP%20P%20Plankton))
  (bind _returnvalue (== OtherActor _as_bp_p_plankton))
  (if _returnvalue
    (Variables|Default|SetNewVar_0 _returnvalue)
    (Development|PrintString "Bss Time")
    (Utilities|FlowControl|Sequence
      (:then_0
        (bind _asboss_chase (Utilities|Casting|CastToBoss_Chase (Components|GetOwner)))
        (Variables|/Game/BP/Enemy/FakeBoss/Boss_Chase.Boss_Chase_C|SetEvent%20End _asboss_chase true))
      (:then_1
        (Utilities|FlowControl|Delay 0.2)
        (Game|OpenLevel(byObjectReference) "/Game/Level/Berni_BossLevel.Berni_BossLevel")))))

(event EventBeginPlay
  (bind _asbp_p_plankton (Utilities|Casting|CastToBP_P_Plankton (Game|Player|GetPlayerPawn 0)))
  (Variables|Default|SetAs%20BP%20P%20Plankton _asbp_p_plankton))

(event EventTick
  (params (DeltaSeconds :type Float%20%28single-precision%29))
  (if (Variables|Default|GetNewVar_0)
    (bind _asbp_p_plankton (Utilities|Casting|CastToBP_P_Plankton (Game|Player|GetPlayerPawn 0)))
    (Variables|/Game/BP/PC_Pawn/BP_P_Plankton.BP_P_Plankton_C|SetMaxVelocity _asbp_p_plankton "0, 0, 0")
    (Variables|/Game/BP/PC_Pawn/BP_P_Plankton.BP_P_Plankton_C|SetAddVelocity _asbp_p_plankton "0, 0, 0")))

(fn ConstructionScript)