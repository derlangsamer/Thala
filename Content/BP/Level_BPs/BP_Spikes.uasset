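; BP_Spikes is a level hazard that knocks back and damages the player's Plankton pawn on contact.
; It caches the player pawn on BeginPlay, then reacts only when that pawn's Painbox overlaps Box1.
; The Arrow's world location becomes the knockback origin before StartKnockBack is called.
; Damage is applied by finding every Char_Health_Component actor in the world and calling Damage on each.
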(event OnComponentBeginOverlap(Box1)
  (params (OverlappedComponent :type Primitive%20Component%20Object%20Reference) (OtherActor :type Actor%20Object%20Reference) (OtherComp :type Primitive%20Component%20Object%20Reference) (OtherBodyIndex :type Integer) (bFromSweep :type Boolean) (SweepResult :type Hit%20Result%20Structure%20%28by%20ref%29))
  (if (== OtherActor (Variables|Default|GetAs%20BP%20P%20Plankton))
    (if (== OtherComp (Variables|/Game/BP/PC_Pawn/BP_P_Plankton.BP_P_Plankton_C|GetPainbox (Variables|Default|GetAs%20BP%20P%20Plankton)))
      (Variables|/Game/BP/PC_Pawn/BP_P_Plankton.BP_P_Plankton_C|SetKnockbackOrigin (Variables|Default|GetAs%20BP%20P%20Plankton) (Transformation|GetWorldLocation (Variables|Default|GetArrow)))
      (Default|StartKnockBack (Variables|Default|GetAs%20BP%20P%20Plankton))
      (bind _outactors (Actor|GetAllActorsOfClass "/Game/BP/Health_UI/Health_Ui/Health_System/Char_Health_Component.Char_Health_Component_C"))
      (for _array_element _outactors
        (bind _aschar_health_component (Utilities|Casting|CastToChar_Health_Component _array_element))
        (Default|Damage _aschar_health_component)))))

(event EventBeginPlay
  (bind _asbp_p_plankton (Utilities|Casting|CastToBP_P_Plankton (Game|Player|GetPlayerPawn 0)))
  (Variables|Default|SetAs%20BP%20P%20Plankton _asbp_p_plankton))

(fn ConstructionScript)