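; BP_Target is a harpoon target that creates a rock bridge when hit.
; On overlap with a BP_Harpoon, it spawns BP_RockBridge at a fixed offset along Y and below its Target component.
; The DidISpawn counter guards against repeat spawns, and the actor destroys itself after spawning the bridge.
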(event EventBeginPlay)

(event Collision|EventActorBeginOverlap
  (params (OtherActor :type Actor%20Object%20Reference))
  (bind _target (Variables|Default|GetTarget))
  (bind _returnvalue (Transformation|GetWorldLocation _target))
  (bind (_x _y _z) (Math|Vector|BreakVector _returnvalue))
  (Utilities|Casting|CastToBP_Harpoon OtherActor)
  (if (< (Variables|Default|GetDidISpawn) 1)
    (Game|SpawnActorfromClass "/Game/BP/Level_BPs/RockBridge/BP_RockBridge.BP_RockBridge_C" (Math|Conversions|ToTransform(Vector) (Math|Vector|MakeVector _x (+ _y 5.5e+02) (- _z 3e+02))) "Undefined" 0 0)
    (bind _output_get (Variables|Default|SetDidISpawn (+ (stale _output_get) 1)))
    (Actor|DestroyActor)))

(event EventTick
  (params (DeltaSeconds :type Float%20%28single-precision%29)))

(fn ConstructionScript)